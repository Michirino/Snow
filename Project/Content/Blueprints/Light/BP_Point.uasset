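; BP_Point is a point light actor that fades out when the player reaches it.
; BeginPlay sets the light to full brightness.
; When BP_Player overlaps the Sphere component, a timeline plays and each update lerps the light's current intensity toward zero, so the fade compounds from the live value rather than the starting one.
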(event `self.ReceiveBeginPlay`
  (`LightComponent.SetIntensity` (`self.PointLight`) 1000.0))

(event `self.Sphere.OnComponentBeginOverlap`
  (params (OverlappedComponent :type "PrimitiveComponent Object Reference") (OtherActor :type "Actor Object Reference") (OtherComp :type "PrimitiveComponent Object Reference") (OtherBodyIndex :type Integer) (bFromSweep :type Boolean) (SweepResult :type "HitResult Structure (by ref)"))
  (bind _asbp_third_person_character (cast `/Game/ThirdPerson/Blueprints/BP_Player` OtherActor))
  (if (== _asbp_third_person_character OtherActor)
    (bind (_direction _newtrack_0) (`Timeline|Timeline_0`)
      (:`Update`
        (`LightComponent.SetIntensity` (`self.PointLight`) (`KismetMathLibrary.Lerp` (`LightComponentBase.Intensity` (`self.PointLight`)) 0.0 _newtrack_0))))))

(fn `UserConstructionScript`)