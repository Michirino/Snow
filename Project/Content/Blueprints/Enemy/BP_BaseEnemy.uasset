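; Base enemy Blueprint, apparently a zombie, that chases the player, plays random attack montages, reacts to damage and dies.
; CharcingPlayer and SmartAttacking loop through AI MoveTo and attacks, using randomness, an attack counter and attack-range overlap to decide when to pause.
; Leaving the chase radius triggers gated, delayed Waiting, which returns it to spawn unless interrupted.
; OnHIt reduces health, then resumes attacking or calls Daying, which disables mesh collision.
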(event `self.ReceiveBeginPlay`
  (`self.Inisetalation`)
  (set `self.Spawnpoint` (`SceneComponent.K2_GetComponentLocation` (`self.Mesh`))))

(event `Waiting`
  (`|ExecutionSequence`
    (:`then_0`
      (`self.AttackPause`)
      (`KismetSystemLibrary.Delay` 10.0)
      (`/Engine/EditorBlueprintResources/StandardMacros.Gate` true :!label _label
        (:`Exit`
          (`|AIMoveTo` self (`self.Spawnpoint`) null))))
    (:`then_1`
      (goto _label :!via `Open`))))

(event `AttackPause`
  (set `self.AttackMode` false)
  (set `self.CanAttack?` false)
  (`self.StopMoving`)
  (`KismetSystemLibrary.Delay` 2.0)
  (set `self.AttackCounter` 0)
  (set `self.CanAttack?` true))

(event `CharcingPlayer`
  (bind _attackmontages (`self.AttackMontages`))
  (`|ExecutionSequence`
    (:`then_0`
      (`KismetSystemLibrary.Delay` 0.0001)
      (`KismetSystemLibrary.PrintString` "thinking")
      (if (not (`self.IsDeath`))
        (if (`self.CanAttack?`)
          (`/Engine/EditorBlueprintResources/StandardMacros.IncrementInt` (`self.AttackCounter`)
            (:`  `
              (if (>= (`self.AttackCounter`) 4)
                (if (not (`self.InnAttackRadius`))
                  (set `self.AttackMode` false))
                (else
                  (set `self.AttackMode` true)))
              (`|AIMoveTo` self (0.0 0.0 0.0) (`GameplayStatics.GetPlayerCharacter` 0) 5.0 true
                (:`OnSuccess`
                  (bind _returnvalue (`self.PlayAnimMontage` (`|GetArrayItem` _attackmontages (`KismetMathLibrary.RandomIntegerInRange` 0 (- (`KismetArrayLibrary.Array_Length` _attackmontages) 1)))))
                  (`KismetSystemLibrary.Delay` _returnvalue)
                  (`self.SmartAttacking`))))))))
    (:`then_1`
      (goto _label :!via `Close`))))

(event `SmartAttacking`
  (bind _output_get (set `self.AttackNumber` (`KismetMathLibrary.RandomIntegerInRange` 0 4)))
  (if (and (not (== _output_get 1)) (`self.AttackMode`))
    (`self.CharcingPlayer` :!label _label_2)
    (`KismetSystemLibrary.PrintString` "aaaaaa")
    (elif (`self.InnAttackRadius`)
      (goto _label_2)
      (else
        (`self.AttackPause`)
        (`KismetSystemLibrary.PrintString` "pause")))))

(event `OnHIt`
  (params (Damage :type "Float (double-precision)"))
  (bind _health (`self.Health`))
  (`self.StopMoving`)
  (set `self.Health` (- _health Damage))
  (if (<= _health 0.0)
    (`self.Daying`)
    (else
      (bind _returnvalue (`self.PlayAnimMontage` "/Game/Animations/Enemy/Animations/OnHIt/ZombyOnHit.ZombyOnHit"))
      (`KismetSystemLibrary.Delay` _returnvalue)
      (`self.SmartAttacking`))))

(event `Daying`
  (set `self.AttackMode` false)
  (set `self.IsDeath` true)
  (`self.StopMoving`)
  (`self.PlayAnimMontage` "/Game/Animations/Enemy/Animations/OnHIt/Daying.Daying")
  (`PrimitiveComponent.SetCollisionResponseToAllChannels` (`self.Mesh`) "ECR_Ignore"))

(event `self.AttackRange.OnComponentBeginOverlap`
  (params (OverlappedComponent :type "PrimitiveComponent Object Reference") (OtherActor :type "Actor Object Reference") (OtherComp :type "PrimitiveComponent Object Reference") (OtherBodyIndex :type Integer) (bFromSweep :type Boolean) (SweepResult :type "HitResult Structure (by ref)"))
  (bind _asbp_third_person_character (cast `/Game/ThirdPerson/Blueprints/BP_Player` OtherActor))
  (set `self.Player` _asbp_third_person_character)
  (`/Engine/EditorBlueprintResources/StandardMacros.IsValid` _asbp_third_person_character
    (:`Is Valid`
      (set `self.InnAttackRadius` true))))

(event `self.AttackRange.OnComponentEndOverlap`
  (params (OverlappedComponent :type "PrimitiveComponent Object Reference") (OtherActor :type "Actor Object Reference") (OtherComp :type "PrimitiveComponent Object Reference") (OtherBodyIndex :type Integer))
  (bind _player (`self.Player`)
    (:`then`
      (if (== OtherActor _player)
        (set `self.InnAttackRadius` false)))
    (:`else`)))

(event `self.ChacingRadius.OnComponentBeginOverlap`
  (params (OverlappedComponent :type "PrimitiveComponent Object Reference") (OtherActor :type "Actor Object Reference") (OtherComp :type "PrimitiveComponent Object Reference") (OtherBodyIndex :type Integer) (bFromSweep :type Boolean) (SweepResult :type "HitResult Structure (by ref)"))
  (bind _asbp_third_person_character (cast `/Game/ThirdPerson/Blueprints/BP_Player` OtherActor))
  (set `self.Player` _asbp_third_person_character)
  (`/Engine/EditorBlueprintResources/StandardMacros.IsValid` _asbp_third_person_character
    (:`Is Valid`
      (`KismetSystemLibrary.PrintString` "inradius")
      (goto _label_3 :!via `Close`))))

(event `self.ChacingRadius.OnComponentEndOverlap`
  (params (OverlappedComponent :type "PrimitiveComponent Object Reference") (OtherActor :type "Actor Object Reference") (OtherComp :type "PrimitiveComponent Object Reference") (OtherBodyIndex :type Integer))
  (`KismetSystemLibrary.PrintString` "leafe radius")
  (bind _player (`self.Player`)
    (:`then`
      (if (== OtherActor _player)
        (`|ExecutionSequence`
          (:`then_0`
            (`KismetSystemLibrary.Delay` (`self.PlayerTrackTime`))
            (`/Engine/EditorBlueprintResources/StandardMacros.Gate` true :!label _label_3
              (:`Exit`
                (`self.Waiting`))))
          (:`then_1`
            (goto _label_3 :!via `Open`)))))
    (:`else`)))

(fn `AttackPlayer`)

(fn `Death`
  (`self.K2_DestroyActor`))

(fn `Inisetalation`
  (`SphereComponent.SetSphereRadius` (`self.AttackRange`) (`self.AttackRadius`) true)
  (`SphereComponent.SetSphereRadius` (`self.LookAtRadius`) (`self.LookAt`) true))

(fn `StopMoving`
  (`MovementComponent.StopMovementImmediately` (`self.CharacterMovement`)))

(fn `UserConstructionScript`)