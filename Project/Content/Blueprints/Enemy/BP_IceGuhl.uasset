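; BP_IceGuhl is an enemy ghoul that starts with an ice sound and charges the player who enters its LookAtRadius sphere.
; If iced, it first stops that sound, runs BreakIce for an explosion effect and material swap, screams, and resizes the sphere to its no-ice radius.
; It waits out the scream montage before charging, while any damage received is passed to OnHIt.
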(event `self.ReceiveBeginPlay`
  (`parent.ReceiveBeginPlay`)
  (bind _returnvalue (`GameplayStatics.SpawnSoundAtLocation` "/Game/Sounds/SQ/Enemy/SQ_GuhlIce.SQ_GuhlIce" (`SceneComponent.K2_GetComponentLocation` (`self.Mesh`)) (struct) 1.0 1.0 0.0 null null)))

(event `self.LookAtRadius.OnComponentBeginOverlap`
  (params (OverlappedComponent :type "PrimitiveComponent Object Reference") (OtherActor :type "Actor Object Reference") (OtherComp :type "PrimitiveComponent Object Reference") (OtherBodyIndex :type Integer) (bFromSweep :type Boolean) (SweepResult :type "HitResult Structure (by ref)"))
  (bind _asbp_third_person_character (cast `/Game/ThirdPerson/Blueprints/BP_Player` OtherActor))
  (`/Engine/EditorBlueprintResources/StandardMacros.IsValid` _asbp_third_person_character
    (:`Is Valid`
      (set `self.Player_0` _asbp_third_person_character)
      (if (`self.Ice`)
        (`AudioComponent.Stop` (stale `self.ReceiveBeginPlay` _returnvalue))
        (bind _returnvalue (`self.BreakIce`))
        (bind _returnvalue_2 (`self.PlayAnimMontage` "/Game/Animations/Enemy/Animations/MonScreem.MonScreem"))
        (`KismetSystemLibrary.Delay` 0.2)
        (set `self.Ice` false)
        (`GameplayStatics.PlaySoundAtLocation` "/Game/Sounds/SQ/Enemy/SQ_GuhlScreem.SQ_GuhlScreem" _returnvalue (struct) 1.0 1.0 0.0 null null null null)
        (`SphereComponent.SetSphereRadius` (`self.LookAtRadius`) (`self.NoIceLoockAtRadius`) true)
        (`KismetSystemLibrary.Delay` _returnvalue_2)
        (`self.CharcingPlayer`)
        (else
          (`self.CharcingPlayer`))))))

(event `self.ReceiveAnyDamage`
  (params (Damage :type "Float (single-precision)") (DamageType :type "DamageType Object Reference") (InstigatedBy :type "Controller Object Reference") (DamageCauser :type "Actor Object Reference"))
  (`self.OnHIt` Damage))

(fn `BreakIce`
  (returns (ReturnValue :type "Vector Structure"))
  (bind _returnvalue (`SceneComponent.K2_GetComponentLocation` (`self.Mesh`)))
  (set `self.Ice` false)
  (`GameplayStatics.SpawnEmitterAtLocation` "/Game/StarterContent/Particles/P_IceExplosion.P_IceExplosion" (`SceneComponent.K2_GetComponentLocation` (`self.Mesh`)) (struct) (2.0 2.0 2.0))
  (for _index (range 3)
    (`PrimitiveComponent.SetMaterial` (`self.Mesh`) _index (`|GetArrayItem` (`self.Material`) _index)))
  (`GameplayStatics.PlaySoundAtLocation` "/Game/Sounds/SQ/Enemy/SQ_EnemyIceExplosion.SQ_EnemyIceExplosion" _returnvalue (struct) 1.0 1.0 0.0 null null null null)
  (return _returnvalue))

(fn `UserConstructionScript`
  (`parent.UserConstructionScript`))