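; Base equippable item that tracks its equipped state and attaches to the owning Character's mesh.
; Equipping sets the flag and snaps the item to a configurable socket, keeping relative scale.
; Unequipping only clears the flag, without detaching.
; A mesh getter returns the static mesh component if it has a valid asset, otherwise the skeletal one.
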(fn `AttatchToActor`
  (params (SocketName :type Name))
  (`self.K2_AttachToComponent` (`Character.Mesh` (cast `Character` (`self.GetOwner`) :!pure true)) SocketName "SnapToTarget" "SnapToTarget" "KeepRelative"))

(fn `GetItemMesh`
  (returns (ReturnValue :type "PrimitiveComponent Object Reference"))
  (`/Engine/EditorBlueprintResources/StandardMacros.IsValid` (`StaticMeshComponent.StaticMesh` (`self.StaticMesh`))
    (:`Is Valid`
      (return (`self.StaticMesh`)))
    (:`Is Not Valid`
      (return (`self.SkeletalMesh`)))))

(fn `IsEpuipped`
  (returns (`IsEquipped?` :type Boolean))
  (return (`self.IsEquipped?`)))

(fn `OnEquipped`
  (set `self.IsEquipped?` true)
  (`self.AttatchToActor` (`self.AttatchSoketName`)))

(fn `OnUnequipped`
  (if (`self.IsEquipped?`)
    (set `self.IsEquipped?` false)))

(fn `SetIsEquipped`
  (params (`IsEquipped?` :type Boolean))
  (set `self.IsEquipped?` `IsEquipped?`))

(fn `UserConstructionScript`)